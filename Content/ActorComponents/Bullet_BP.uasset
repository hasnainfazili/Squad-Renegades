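; Projectile Blueprint that explodes on hit, dealing radial rocket damage.
; The Hit event calls a server-named event, which forwards to an RPC event that does all the explosion work.
; That event applies damage at the hit location using ImpulseForce as the radius, then spawns a scaled explosion emitter and plays a hitmarker sound.
; It also adds a new Hitmarker widget to the viewport, without checking what was hit.
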(event `Radial_Serever`
  (`self.RPC_Radial`))

(event `RPC_Radial`
  (bind (_bblockinghit _binitialoverlap _time _distance _location) (`GameplayStatics.BreakHitResult` (stale `self.ReceiveHit` Hit)))
  (`GameplayStatics.ApplyRadialDamage` :`BaseDamage` (`self.Damage`) :`Origin` _location :`DamageRadius` (`self.Impulse Force`) :`DamageTypeClass` "/Game/ActorComponents/RocketDamageType.RocketDamageType_C" :`DamageCauser` null :`InstigatedByController` null)
  (`GameplayStatics.SpawnEmitterAtLocation` "/Game/StarterContent/Particles/P_Explosion.P_Explosion" _location (struct) (3.0 3.0 3.0))
  (`GameplayStatics.PlaySoundAtLocation` "/Game/SFX/Voicy_The_Last_Of_Us_Hitmarker_Sound.Voicy_The_Last_Of_Us_Hitmarker_Sound" _location (struct) 1.0 1.0 0.0 null null null null)
  (bind _returnvalue (`|CreateWidget` "/Game/ActorComponents/Hitmarker.Hitmarker_C"))
  (`UserWidget.AddToViewport` _returnvalue 0))

(event `self.ReceiveHit`
  (params (MyComp :type "PrimitiveComponent Object Reference") (Other :type "Actor Object Reference") (OtherComp :type "PrimitiveComponent Object Reference") (bSelfMoved :type Boolean) (HitLocation :type "Vector Structure") (HitNormal :type "Vector Structure") (NormalImpulse :type "Vector Structure") (Hit :type "HitResult Structure (by ref)"))
  (`self.Radial_Serever`))

(fn `UserConstructionScript`)